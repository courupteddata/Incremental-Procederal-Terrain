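; Procedural terrain actor that builds a noise-displaced grid mesh with collision in its construction script.
; One loop lays out RowX by RowY quads, setting each vertex height from seeded 2D noise and filling UV and triangle arrays.
; Smooth normals sum area-scaled face normals at each vertex, multiplied by all three triangle angles, then normalize.
; The arrays feed a ProceduralMesh section using a color grid material.
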(event EventBeginPlay)

(event Collision|EventActorBeginOverlap
  (params (OtherActor :type Actor%20Object%20Reference)))

(event EventTick
  (params (DeltaSeconds :type Float%20%28single-precision%29)))

(fn ConstructionScript
  (bind _normals (Variables|Default|GetNormals))
  (bind _triangles (Variables|Default|GetTriangles))
  (bind _proceduralmesh (Variables|Default|GetProceduralMesh))
  (bind _rowx (Variables|Default|GetRowX))
  (bind _normals_2 (Variables|Default|GetNormals))
  (bind _polysize (Variables|Default|GetPolySize))
  (bind _rowx_2 (Variables|Default|GetRowX))
  (bind _triangles_2 (Variables|Default|GetTriangles))
  (bind _vertices (Variables|Default|GetVertices))
  (bind _returnvalue (+ _rowx_2 1))
  (Rendering|Material|SetMaterial _proceduralmesh 0 "/Game/StarterContent/Materials/M_ColorGrid_LowSpec.M_ColorGrid_LowSpec")
  ;[1 1 1] Loop Section
  (for _index (range 0 (- (* (+ (Variables|Default|GetRowY) 1) (+ (Variables|Default|GetRowX) 1)) 1))
    (bind _returnvalue_2 (Class|UFNNoiseGenerator|GetNoise2D (Class|UFNBlueprintFunctionLibrary|CreateSimpleNoiseGenerator _proceduralmesh (Variables|Default|GetNoiseType) (Variables|Default|GetSeed) (Variables|Default|GetFrequency) (Variables|Default|GetInterpolation)) (.X (Math|Vector|BreakVector (+ (Variables|Default|GetLocation) (Math|Vector|MakeVector _polysize 0.0 0.0)))) (.Y (Math|Vector|BreakVector (+ (Variables|Default|GetLocation) (Math|Vector|MakeVector _polysize 0.0 0.0))))))
    (if (== (Math|Integer|%(Integer) (+ _index 1) (+ (Variables|Default|GetRowX) 1)) 0)
      ;[1 1 1] Vertices Creation
      (bind _output_get (Variables|Default|SetLocation (+ (Variables|Default|GetLocation) (Math|Vector|MakeVector _polysize 0.0 0.0))))
      (Utilities|Array|Add (Variables|Default|GetVertices) (Math|Vector|MakeVector (.X (Math|Vector|BreakVector _output_get)) (.Y (Math|Vector|BreakVector _output_get)) (* _polysize _returnvalue_2)))
      (Variables|Default|SetLocation (+ (Variables|Default|GetLocation) (Math|Vector|MakeVector (* (* _polysize (Math|Conversions|ToFloat(Integer) (+ (Variables|Default|GetRowX) 1))) -1.0) _polysize 0.0)))
      (else
        (bind _output_get_2 (Variables|Default|SetLocation (+ (Variables|Default|GetLocation) (Math|Vector|MakeVector _polysize 0.0 0.0))))
        (Utilities|Array|Add (Variables|Default|GetVertices) (Math|Vector|MakeVector (.X (Math|Vector|BreakVector _output_get_2)) (.Y (Math|Vector|BreakVector _output_get_2)) (* _polysize _returnvalue_2)))))
    ;[1 1 1] UV  Section
    (if (Variables|Default|GetRoot)
      (bind _output_get_3 (Variables|Default|SetUV0 ""))
      (Utilities|Array|Add (Variables|Default|GetUV) _output_get_3)
      (Variables|Default|SetRoot false)
      (elif (== (Math|Integer|%(Integer) (+ _index 0) (+ (Variables|Default|GetRowX) 1)) 0)
        (Utilities|Array|Add (Variables|Default|GetUV) (+ (Variables|Default|GetUV0) (Math|Vector2D|MakeVector2D -1.0 (/ 1.0 (Math|Conversions|ToFloat(Integer) (Variables|Default|GetRowY))))))
        (Variables|Default|SetUV0 (+ (Variables|Default|GetUV0) (Math|Vector2D|MakeVector2D -1.0 (/ 1.0 (Math|Conversions|ToFloat(Integer) (Variables|Default|GetRowY))))))
        (else
          (bind _output_get_4 (Variables|Default|SetUV0 (+ (Variables|Default|GetUV0) (Math|Vector2D|MakeVector2D (/ 1.0 (Math|Conversions|ToFloat(Integer) (Variables|Default|GetRowX))) 0.0))))
          (Utilities|Array|Add (Variables|Default|GetUV) _output_get_4))))
    ;[1 1 1] Triangle Section
    (if (not (== (Math|Integer|%(Integer) (+ _index 1) (+ (Variables|Default|GetRowX) 1)) 0))
      (if (== (- (- (* (+ _rowx 1) (+ (Variables|Default|GetRowY) 1)) 1) _rowx) _index)
        (Variables|Default|SetCreateTriangle false)
        (elif (Variables|Default|GetCreateTriangle)
          (Utilities|Array|Insert _triangles _index (Variables|Default|GetTriangleArrayLocation))
          (Utilities|Array|Insert _triangles (+ _index _returnvalue) (+ (Variables|Default|GetTriangleArrayLocation) 1))
          (Utilities|Array|Insert _triangles (+ _index 1) (+ (+ (Variables|Default|GetTriangleArrayLocation) 1) 1))
          (Utilities|Array|Insert _triangles (+ _index 1) (+ (+ (+ (Variables|Default|GetTriangleArrayLocation) 1) 1) 1))
          (Utilities|Array|Insert _triangles (+ _index _returnvalue) (+ (+ (+ (+ (Variables|Default|GetTriangleArrayLocation) 1) 1) 1) 1))
          (Utilities|Array|Insert _triangles (+ (+ _returnvalue 1) _index) (+ (+ (+ (+ (+ (Variables|Default|GetTriangleArrayLocation) 1) 1) 1) 1) 1))
          (Variables|Default|SetTriangleArrayLocation (+ (+ (+ (+ (+ (+ (Variables|Default|GetTriangleArrayLocation) 1) 1) 1) 1) 1) 1))))))
  ;[1 1 1] Initializing normals array
  (for _index_2 (range 0 (Utilities|Array|LastIndex (Variables|Default|GetVertices)))
    (Utilities|Array|Add :TargetArray (Variables|Default|GetNormals)))
  (for _index_3 (range 0 (Utilities|Array|LastIndex (Variables|Default|GetTriangles)))
    ;[1 1 1] Compute Vertex normals
    (if (== (Math|Integer|%(Integer) _index_3 3) 0)
      (bind (_area _normal) (CallFunction|TriangleAreaandNormal (Utilities|Array|Get(acopy) _vertices (Utilities|Array|Get(acopy) _triangles_2 _index_3)) (Utilities|Array|Get(acopy) _vertices (Utilities|Array|Get(acopy) _triangles_2 (+ _index_3 1))) (Utilities|Array|Get(acopy) _vertices (Utilities|Array|Get(acopy) _triangles_2 (+ (+ _index_3 1) 1)))))
      (bind (_anglea _angleb _anglec) (CallFunction|ThreeAngles (Utilities|Array|Get(acopy) _vertices (Utilities|Array|Get(acopy) _triangles_2 _index_3)) (Utilities|Array|Get(acopy) _vertices (Utilities|Array|Get(acopy) _triangles_2 (+ _index_3 1))) (Utilities|Array|Get(acopy) _vertices (Utilities|Array|Get(acopy) _triangles_2 (+ (+ _index_3 1) 1)))))
      (Utilities|FlowControl|Sequence
        (:then_0
          (Utilities|Array|SetArrayElem _normals (Utilities|Array|Get(acopy) _triangles_2 _index_3) (+ (Utilities|Array|Get(acopy) _normals (Utilities|Array|Get(acopy) _triangles_2 _index_3)) (+ (* (* _normal _area) _angleb) (* (* _normal _area) _anglea) (* (* _normal _area) _anglec)))))
        (:then_1
          (Utilities|Array|SetArrayElem _normals (Utilities|Array|Get(acopy) _triangles_2 (+ _index_3 1)) (+ (Utilities|Array|Get(acopy) _normals (Utilities|Array|Get(acopy) _triangles_2 (+ _index_3 1))) (+ (* (* _normal _area) _angleb) (* (* _normal _area) _anglea) (* (* _normal _area) _anglec)))))
        (:then_2
          (Utilities|Array|SetArrayElem _normals (Utilities|Array|Get(acopy) _triangles_2 (+ (+ _index_3 1) 1)) (+ (Utilities|Array|Get(acopy) _normals (Utilities|Array|Get(acopy) _triangles_2 (+ (+ _index_3 1) 1))) (+ (* (* _normal _area) _angleb) (* (* _normal _area) _anglea) (* (* _normal _area) _anglec))))))))
  ;[1 1 1] Normalizing vertex normals
  (for (_array_element _array_index) _normals_2
    (Utilities|Array|SetArrayElem _normals_2 _array_index (Math|Vector|Normalize _array_element)))
  ;[1 1 1] Create Section
  (Class|ProceduralMeshComponent|CreateMeshSectionLinearColor (Variables|Default|GetProceduralMesh) 0 (Variables|Default|GetVertices) (Variables|Default|GetTriangles) (Variables|Default|GetNormals) (Variables|Default|GetUV) 0 0 true))