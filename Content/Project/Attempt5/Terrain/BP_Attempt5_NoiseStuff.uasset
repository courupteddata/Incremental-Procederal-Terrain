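; Blueprint noise helper in the Attempt5 terrain folder that provides a Pattern function returning one domain-warped 2D fractal noise value for a point.
; Two offset FBM samples form vector Q, which displaces the point for a second pair forming R, which warps the final sample.
; Each of the five samples creates its own generator from the same caller-supplied noise type, seed, frequency and fractal settings.
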(fn Pattern
  (params (Outer :type Object%20Object%20Reference) (P :type Vector%202D%20Structure) (Octaves :type Integer) (Lacunarity :type Float%20%28single-precision%29) (FractalGain :type Float%20%28single-precision%29) (Frequency :type Float%20%28single-precision%29) (NoiseType :type EFractalNoiseType%20Enum :default "FractalValue") (Seed :type Integer) (Interpolation :type EInterp%20Enum :default "InterpLinear"))
  (bind _returnvalue (Class|UFNBlueprintFunctionLibrary|CreateFractalNoiseGenerator Outer NoiseType Seed Frequency FractalGain Interpolation "FBM" Octaves Lacunarity))
  (bind (_x _y) (Math|Vector2D|BreakVector2D P))
  (bind _returnvalue_2 (+ P "(X=5.200000,Y=1.300000)"))
  (bind (_x_2 _y_2) (Math|Vector2D|BreakVector2D _returnvalue_2))
  (bind _returnvalue_3 (Class|UFNNoiseGenerator|GetNoise2D _returnvalue _x _y))
  (bind _returnvalue_4 (Class|UFNNoiseGenerator|GetNoise2D _returnvalue _x_2 _y_2))
  (bind _output_get (LocalVariables|Setq (Math|Vector2D|MakeVector2D _returnvalue_3 _returnvalue_4)))
  (bind _returnvalue_5 (Class|UFNNoiseGenerator|GetNoise2D _returnvalue (.X (Math|Vector2D|BreakVector2D (+ P (+ (* _output_get 4.0) "(X=1.700000,Y=9.200000)")))) (.Y (Math|Vector2D|BreakVector2D (+ P (+ (* _output_get 4.0) "(X=1.700000,Y=9.200000)"))))))
  (bind _returnvalue_6 (Class|UFNNoiseGenerator|GetNoise2D _returnvalue (.X (Math|Vector2D|BreakVector2D (+ P (+ (* _output_get 4.0) "(X=8.300000,Y=2.800000)")))) (.Y (Math|Vector2D|BreakVector2D (+ P (+ (* _output_get 4.0) "(X=8.300000,Y=2.800000)"))))))
  (bind _output_get_2 (LocalVariables|Setr (Math|Vector2D|MakeVector2D _returnvalue_5 _returnvalue_6)))
  (bind _returnvalue_7 (Class|UFNNoiseGenerator|GetNoise2D _returnvalue (.X (Math|Vector2D|BreakVector2D (+ (* _output_get_2 4.0) P))) (.Y (Math|Vector2D|BreakVector2D (+ (* _output_get_2 4.0) P)))))
  (return _returnvalue_7))