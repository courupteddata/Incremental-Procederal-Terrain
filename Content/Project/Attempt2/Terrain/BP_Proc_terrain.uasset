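; BP_Proc_terrain is a procedural terrain actor that builds a randomly bumpy grid mesh in its Construction Script.
; A single loop over RowX+1 by RowY+1 points lays out PolySize-spaced vertices with random Z offsets, accumulates normalized UVs and inserts two triangles per cell.
; The arrays feed one ProceduralMesh section with collision and a color-grid material.
; Heights use unseeded random calls, and the event graph is empty.
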(event EventBeginPlay)

(event Collision|EventActorBeginOverlap
  (params (OtherActor :type Actor%20Object%20Reference)))

(event EventTick
  (params (DeltaSeconds :type Float%20%28single-precision%29)))

(fn ConstructionScript
  (bind _triangles (Variables|Default|GetTriangles))
  (bind _rowx (Variables|Default|GetRowX))
  (bind _polysize (Variables|Default|GetPolySize))
  (bind _rowx_2 (Variables|Default|GetRowX))
  (bind _returnvalue (+ _rowx_2 1))
  (Rendering|Material|SetMaterial (Variables|Default|GetProceduralMesh) 0 "/Game/StarterContent/Materials/M_ColorGrid_LowSpec.M_ColorGrid_LowSpec")
  ;[1 1 1] Loop Section
  (for _index (range 0 (- (* (+ (Variables|Default|GetRowY) 1) (+ (Variables|Default|GetRowX) 1)) 1))
    (if (== (Math|Integer|%(Integer) (+ _index 1) (+ (Variables|Default|GetRowX) 1)) 0)
      ;[1 1 1] Vertices Creation
      (bind _output_get (Variables|Default|SetLocation (+ (Variables|Default|GetLocation) (Math|Vector|MakeVector _polysize 0.0 0.0))))
      (Utilities|Array|Add (Variables|Default|GetVertices) (Math|Vector|MakeVector (.X (Math|Vector|BreakVector _output_get)) (.Y (Math|Vector|BreakVector _output_get)) (* _polysize (Math|Random|RandomFloatinRange -0.5 0.5))))
      (Variables|Default|SetLocation (+ (Variables|Default|GetLocation) (Math|Vector|MakeVector (* (* _polysize (Math|Conversions|ToFloat(Integer) (+ (Variables|Default|GetRowX) 1))) -1.0) _polysize 0.0)))
      (else
        (bind _output_get_2 (Variables|Default|SetLocation (+ (Variables|Default|GetLocation) (Math|Vector|MakeVector _polysize 0.0 0.0))))
        (Utilities|Array|Add (Variables|Default|GetVertices) (Math|Vector|MakeVector (.X (Math|Vector|BreakVector _output_get_2)) (.Y (Math|Vector|BreakVector _output_get_2)) (* _polysize (Math|Random|RandomFloatinRange -0.5 0.5))))))
    ;[1 1 1] UV  Section
    (if (Variables|Default|GetRoot)
      (bind _output_get_3 (Variables|Default|SetUV0 ""))
      (Utilities|Array|Add (Variables|Default|GetUV) _output_get_3)
      (Variables|Default|SetRoot false)
      (elif (== (Math|Integer|%(Integer) (+ _index 0) (+ (Variables|Default|GetRowX) 1)) 0)
        (Utilities|Array|Add (Variables|Default|GetUV) (+ (Variables|Default|GetUV0) (Math|Vector2D|MakeVector2D -1.0 (/ 1.0 (Math|Conversions|ToFloat(Integer) (Variables|Default|GetRowY))))))
        (Variables|Default|SetUV0 (+ (Variables|Default|GetUV0) (Math|Vector2D|MakeVector2D -1.0 (/ 1.0 (Math|Conversions|ToFloat(Integer) (Variables|Default|GetRowY))))))
        (else
          (bind _output_get_4 (Variables|Default|SetUV0 (+ (Variables|Default|GetUV0) (Math|Vector2D|MakeVector2D (/ 1.0 (Math|Conversions|ToFloat(Integer) (Variables|Default|GetRowX))) 0.0))))
          (Utilities|Array|Add (Variables|Default|GetUV) _output_get_4))))
    ;[1 1 1] Triangle Section
    (if (not (== (Math|Integer|%(Integer) (+ _index 1) (+ (Variables|Default|GetRowX) 1)) 0))
      (if (== (- (- (* (+ _rowx 1) (+ (Variables|Default|GetRowY) 1)) 1) _rowx) _index)
        (Variables|Default|SetCreateTriangle false)
        (elif (Variables|Default|GetCreateTriangle)
          (Utilities|Array|Insert _triangles _index (Variables|Default|GetTriangleArrayLocation))
          (Utilities|Array|Insert _triangles (+ _index _returnvalue) (+ (Variables|Default|GetTriangleArrayLocation) 1))
          (Utilities|Array|Insert _triangles (+ _index 1) (+ (+ (Variables|Default|GetTriangleArrayLocation) 1) 1))
          (Utilities|Array|Insert _triangles (+ _index 1) (+ (+ (+ (Variables|Default|GetTriangleArrayLocation) 1) 1) 1))
          (Utilities|Array|Insert _triangles (+ _index _returnvalue) (+ (+ (+ (+ (Variables|Default|GetTriangleArrayLocation) 1) 1) 1) 1))
          (Utilities|Array|Insert _triangles (+ (+ _returnvalue 1) _index) (+ (+ (+ (+ (+ (Variables|Default|GetTriangleArrayLocation) 1) 1) 1) 1) 1))
          (Variables|Default|SetTriangleArrayLocation (+ (+ (+ (+ (+ (+ (Variables|Default|GetTriangleArrayLocation) 1) 1) 1) 1) 1) 1))))))
  ;[1 1 1] Create Section
  (Class|ProceduralMeshComponent|CreateMeshSectionLinearColor (Variables|Default|GetProceduralMesh) 0 (Variables|Default|GetVertices) (Variables|Default|GetTriangles) 0 (Variables|Default|GetUV) 0 0 true))