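; Blueprint helper functions for triangle geometry, filed under the Attempt3 terrain work.
; BP_TriangleAreaAndNormal takes three vertices and returns half the edge cross-product length as area, plus a unit normal along (C-A) × (B-A).
; BP_ThreeAngles returns the interior angle at each vertex in degrees, using the arccosine of dot products between normalized edge vectors.
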(fn BPTriangleAreaandNormal
  (params (A :type Vector) (B :type Vector) (C :type Vector))
  (return (* (Math|Vector|VectorLength (Math|Vector|CrossProduct (- B A) (- C A))) 0.5) (Math|Vector|Normalize (Math|Vector|CrossProduct (- A C) (- A B)))))

(fn BPThreeAngles
  (params (A :type Vector) (B :type Vector) (C :type Vector))
  (return (Class|KismetMathLibrary|DegAcos (Math|Vector|DotProduct (Math|Vector|Normalize (- A B)) (Math|Vector|Normalize (- A C)))) (Class|KismetMathLibrary|DegAcos (Math|Vector|DotProduct (Math|Vector|Normalize (- B A)) (Math|Vector|Normalize (- B C)))) (Class|KismetMathLibrary|DegAcos (Math|Vector|DotProduct (Math|Vector|Normalize (- C A)) (Math|Vector|Normalize (- C B))))))